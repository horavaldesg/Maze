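; Map Blueprint for a puzzle level where hitting certain components reveals hidden paths and reaching the goal shows a win message.
; BeginPlay hides stairs, hidden floor and ramp, ground and the YouWin display, disabling collision on the geometry.
; A character hitting the ramp turns it green and swaps a blocking wall for stairs.
; Other wall hits remove that wall, some revealing ground or a ramp, and hitting the sphere shows YouWin.
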(event OnComponentHit(Ramp)
  (params (HitComponent :type Primitive%20Component%20Object%20Reference) (OtherActor :type Actor%20Object%20Reference) (OtherComp :type Primitive%20Component%20Object%20Reference) (NormalImpulse :type Vector :default "0, 0, 0") (Hit :type Hit%20Result%20Structure%20%28by%20ref%29))
  (bind _stairs (Variables|Default|GetStairs))
  (bind _asthird_person_character (Utilities|Casting|CastToThirdPersonCharacter OtherActor))
  (Rendering|Material|CreateDynamicMaterialInstance (Variables|Default|GetRamp) 0 "/Game/Materials/Green.Green" "None" :!class /Script/Engine.PrimitiveComponent)
  (Collision|SetCollisionEnabled (Variables|Default|GetDestroy%20Wall) "NoCollision")
  (Rendering|SetVisibility (Variables|Default|GetDestroy%20Wall) false false)
  (Collision|SetCollisionEnabled _stairs "QueryAndPhysics")
  (Rendering|SetVisibility _stairs true false))

(event OnComponentHit(RightWall)
  (params (HitComponent :type Primitive%20Component%20Object%20Reference) (OtherActor :type Actor%20Object%20Reference) (OtherComp :type Primitive%20Component%20Object%20Reference) (NormalImpulse :type Vector :default "0, 0, 0") (Hit :type Hit%20Result%20Structure%20%28by%20ref%29))
  (bind _hidden_ramp_1 (Variables|Default|GetHidden%20Ramp%201))
  (bind _right_wall (Variables|Default|GetRight%20Wall))
  (Collision|SetCollisionEnabled _right_wall "NoCollision")
  (Rendering|SetVisibility _right_wall false false)
  (Collision|SetCollisionEnabled _hidden_ramp_1 "QueryAndPhysics")
  (Rendering|SetVisibility _hidden_ramp_1 true false))

(event OnComponentHit(Sphere)
  (params (HitComponent :type Primitive%20Component%20Object%20Reference) (OtherActor :type Actor%20Object%20Reference) (OtherComp :type Primitive%20Component%20Object%20Reference) (NormalImpulse :type Vector :default "0, 0, 0") (Hit :type Hit%20Result%20Structure%20%28by%20ref%29))
  (Rendering|SetVisibility (Variables|Default|GetYou%20Win) true false))

(event OnComponentHit(WrongWall)
  (params (HitComponent :type Primitive%20Component%20Object%20Reference) (OtherActor :type Actor%20Object%20Reference) (OtherComp :type Primitive%20Component%20Object%20Reference) (NormalImpulse :type Vector :default "0, 0, 0") (Hit :type Hit%20Result%20Structure%20%28by%20ref%29))
  (bind _wrong_wall (Variables|Default|GetWrong%20Wall))
  (Collision|SetCollisionEnabled _wrong_wall "NoCollision")
  (Rendering|SetVisibility _wrong_wall false false))

(event OnComponentHit(WallRight21)
  (params (HitComponent :type Primitive%20Component%20Object%20Reference) (OtherActor :type Actor%20Object%20Reference) (OtherComp :type Primitive%20Component%20Object%20Reference) (NormalImpulse :type Vector :default "0, 0, 0") (Hit :type Hit%20Result%20Structure%20%28by%20ref%29))
  (bind _wall_right21 (Variables|Default|GetWall%20Right21))
  (bind _ground1 (Variables|Default|GetGround1))
  (Collision|SetCollisionEnabled _wall_right21 "NoCollision")
  (Rendering|SetVisibility _wall_right21 false false)
  (Collision|SetCollisionEnabled _ground1 "QueryAndPhysics")
  (Rendering|SetVisibility _ground1 true false))

(event EventBeginPlay
  (Rendering|SetVisibility (Variables|Default|GetStairs) false false)
  (Collision|SetCollisionEnabled (Variables|Default|GetStairs) "NoCollision"))

(event Collision|EventActorBeginOverlap
  (params (OtherActor :type Actor%20Object%20Reference)))

(event EventTick
  (params (DeltaSeconds :type Float%20%28single-precision%29)))

(fn ConstructionScript)